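; Procedural bookcase that fills five shelves in its Construction Script with random books, potion bottles or both, depending on BookcaseType.
; Static mesh components are packed left to right by bounding-box width until each shelf or random book span is full.
; Bottles get random yaw, a rotation-based margin to trim bounding-box corner waste, and chance-based gaps.
; RandomizeBook varies covers through dynamic material instances setting CoverIndex and a matching MapIndex.
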(fn `RandomizeBook`
  (params (StaticMeshRef :type "StaticMeshComponent Object Reference"))
  (bind _output_get (set `self.CoverIndex` (`KismetMathLibrary.RandomIntegerInRange` 0 4)))
  (switch `int` _output_get
    (:`0`
      (set `self.MapIndex` 2.0 :!label _label))
    (:`1`
      (goto _label))
    (:`2`
      (goto _label))
    (:`3`
      (set `self.MapIndex` 1.0 :!label _label_2))
    (:`4`
      (goto _label_2)))
  (bind _returnvalue (`PrimitiveComponent.CreateDynamicMaterialInstance` StaticMeshRef 0 "/Game/M_imoctezu_Books.M_imoctezu_Books"))
  (`MaterialInstanceDynamic.SetScalarParameterValue` _returnvalue "MapIndex" (`self.MapIndex`))
  (`MaterialInstanceDynamic.SetScalarParameterValue` _returnvalue "CoverIndex" (`KismetMathLibrary.Conv_IntToDouble` (`self.CoverIndex`))))

(fn `UserConstructionScript`
  (bind _returnvalue (`KismetMathLibrary.MakeRotator` 0.0 0.0 90.0))
  (bind _rotation (`self.Rotation`))
  (bind _returnvalue_2 (`KismetMathLibrary.MakeTransform` (0.0 0.0 0.0) _returnvalue (0.6 0.6 0.6)))
  (bind _x (.x (`.BoxExtent` (`KismetSystemLibrary.GetComponentBounds` (`self.ItemBeingPlaced`)))))
  (bind _x_2 (.x (`.BoxExtent` (`KismetSystemLibrary.GetComponentBounds` (`self.ItemBeingPlaced`)))))
  (bind _returnvalue_3 (* _x 2.0))
  (bind _returnvalue_4 (* _x_2 2.0))
  ;[1 1 1] For each shelf
  (for _ (range 5)
    ;[1 1 1] Populate according to Bookcase Type
    (switch `/Game/Enum_imoctezu_BookcaseTypes` (`self.BookcaseType`)
      (:`NewEnumerator0`
        ;[1 0.3979 0.7001] Place Bottles
        ;;[1 1 1] While there is space on the shelf
        (while (< (`self.TotalWidth`) 150.0) :!label _label
          ;;[1 1 1] Randomize rotation for new item
          (bind _output_get (set `self.Rotation` (`KismetMathLibrary.RandomFloatInRange` 0.0 90.0)))
          ;;[1 1 1] Randomize mesh being placed
          (if (> (`KismetMathLibrary.RandomInteger` 100) 50)
            (bind _returnvalue_5 (`KismetMathLibrary.MakeRotator` 0.0 0.0 _output_get))
            (bind _returnvalue_6 (`KismetMathLibrary.MakeTransform` (0.0 0.0 0.0) _returnvalue_5))
            ;;[1 1 1] Create object and save it
            (bind _returnvalue_7 (`AddComponent|NODE_AddStaticMeshComponent-2` :`RelativeTransform` _returnvalue_6))
            (set `self.ItemBeingPlaced` _returnvalue_7)
            (else
              (bind _returnvalue_8 (`AddComponent|NODE_AddStaticMeshComponent-0` :`RelativeTransform` _returnvalue_6))
              (set `self.ItemBeingPlaced` _returnvalue_8)))
          ;;[1 1 1] Figure out size of wasted corner space in bounding box (only useful for round objects)
          ;; [Max waste is at 45 degrees, 0 and 90 have no waste. This formula converts a 0-90 degree value to a 0-45 degree value, since 45+ degrees are a symmetrically flipped version of 0-45 degrees.]
          (if (>= _rotation 45.0)
            (set `self.Margin` (- 90.0 _rotation))
            (else
              (set `self.Margin` _rotation)))
          ;;[1 1 1] Caculate margin adjustment from 5% at 0 to ~-20% at 45
          ;; [This adds a little padding if the objects are not rotated and removes some of the extra corner space if they are.]
          (bind _output_get_2 (set `self.Margin` (* (/ (+ (* (`self.Margin`) -0.4) 2.0) 100.0) _returnvalue_4)))
          ;;[1 1 1] Is there still space for the rotated object?
          (if (<= (+ (`self.TotalWidth`) _returnvalue_4 _output_get_2) 150.0)
            ;;[1 1 1] If yes, decide if it's an object or an object-sized gap
            (if (> (`KismetMathLibrary.RandomFloatInRange` 0.0 100.0) (`self.GapOccurrence`))
              ;;[1 1 1] If it's an object, put it in the right location
              (`SceneComponent.K2_SetRelativeTransform` (`self.ItemBeingPlaced`) (`KismetMathLibrary.MakeTransform` (`KismetMathLibrary.MakeVector` (+ _x_2 (`self.TotalWidth`) (`self.Margin`)) (`KismetMathLibrary.RandomFloatInRange` -8.0 8.0) (`self.CurrentZ`)) _returnvalue_5) false false)
              (else
                ;;[1 1 1] If it's a gap, delete the mesh
                (`ActorComponent.K2_DestroyComponent` (`self.ItemBeingPlaced`))))
            ;;[1 1 1] Add the object/gap width to total
            (set `self.TotalWidth` (+ _returnvalue_4 (`self.TotalWidth`) (* (`self.Margin`) 2.0)))
            (else
              ;;[1 1 1] If not, delete it and break while loop
              (`ActorComponent.K2_DestroyComponent` (`self.ItemBeingPlaced`))
              (set `self.TotalWidth` 9999.0))))
        ;;[1 1 1] When out of space, add Z offset to move to next shelf
        (set `self.CurrentZ` (- (`self.CurrentZ`) 47.5))
        (set `self.TotalWidth` 1.0))
      (:`NewEnumerator1`
        ;[0.1063 0.2664 1] Place Books
        ;;[1 1 1] Tweak the average amount of books being generated based on Bookcase Type
        (set `self.BookSpace` (`KismetMathLibrary.RandomFloatInRange` 60.0 150.0))
        ;;[1 1 1] While there is room in the designated "book space"
        (while (< (`self.TotalWidth`) (`self.BookSpace`)) :!label _label_2
          ;;[1 1 1] Randomize mesh being placed
          (switch `int` (`KismetMathLibrary.RandomIntegerInRange` 0 3)
            (:`0`
              ;;[1 1 1] Create object and save it
              (bind _returnvalue_9 (`AddComponent|NODE_AddStaticMeshComponent-6` :`RelativeTransform` _returnvalue_2))
              (set `self.ItemBeingPlaced` _returnvalue_9))
            (:`1`
              (bind _returnvalue_10 (`AddComponent|NODE_AddStaticMeshComponent-5` :`RelativeTransform` _returnvalue_2))
              (set `self.ItemBeingPlaced` _returnvalue_10))
            (:`2`
              (bind _returnvalue_11 (`AddComponent|NODE_AddStaticMeshComponent-7` :`RelativeTransform` _returnvalue_2))
              (set `self.ItemBeingPlaced` _returnvalue_11))
            (:`3`
              (bind _returnvalue_12 (`AddComponent|NODE_AddStaticMeshComponent-8` :`RelativeTransform` _returnvalue_2))
              (set `self.ItemBeingPlaced` _returnvalue_12)))
          ;;[1 1 1] Randomize book cover
          (`self.RandomizeBook` (`self.ItemBeingPlaced`))
          ;;[1 1 1] Is there still space for the rotated object?
          (if (<= (+ (`self.TotalWidth`) _returnvalue_3 0.0) 150.0)
            ;;[1 1 1] Put it in the right location
            (`SceneComponent.K2_SetRelativeTransform` (`self.ItemBeingPlaced`) (`KismetMathLibrary.MakeTransform` (`KismetMathLibrary.MakeVector` (+ _x (`self.TotalWidth`) (`self.Margin`)) (`KismetMathLibrary.RandomFloatInRange` -2.0 3.0) (`self.CurrentZ`)) _returnvalue (0.6 0.6 0.6)) false false)
            ;;[1 1 1] Add the object width to total
            (set `self.TotalWidth` (+ _returnvalue_3 (`self.TotalWidth`) 0.5))
            (else
              ;;[1 1 1] If not, delete it and break while loop
              (`ActorComponent.K2_DestroyComponent` (`self.ItemBeingPlaced`))
              (set `self.TotalWidth` 9999.0))))
        ;;[1 1 1] If there will be potions after the books, don't move to next shelf
        (if (`|EnumEquality` (`self.BookcaseType`) "NewEnumerator1")
          ;;[1 1 1] When out of space & books only, add Z offset to move to next shelf
          (set `self.CurrentZ` (- (`self.CurrentZ`) 47.5))
          (set `self.TotalWidth` 1.0)))
      (:`NewEnumerator2`
        (`|ExecutionSequence`
          (:`then_0`
            (bind _output_get_3 (set `self.BookSpace` (`KismetMathLibrary.RandomFloatInRange` -20.0 100.0)))
            (if (< _output_get_3 0.0)
              (set `self.BookSpace` 0.0)
              (goto _label_2)
              (else
                (goto _label_2))))
          (:`then_1`
            (goto _label)))))))