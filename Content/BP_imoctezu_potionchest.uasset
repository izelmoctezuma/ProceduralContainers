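; Potion chest Blueprint that procedurally fills itself with a grid of bottle meshes in its Construction Script; the event graph has no active logic.
; Nested loops step through rows and positions, spawning a health or mana bottle by ChestType, with Mixed picking randomly.
; Each bottle gets a random yaw, then is either moved to its slot or destroyed to leave a gap, based on GapOccurrence.
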(fn `UserConstructionScript`
  ;[1 1 1] For every row
  (for _ (range 3)
    ;[1 0.3979 0.7001] Place Bottles
    ;;[1 1 1] For every position in the row
    (for _ (range 7)
      ;;[1 1 1] Randomize rotation for new item
      (bind _output_get (set `self.Rotation` (`KismetMathLibrary.RandomFloatInRange` 60.0 90.0)))
      ;;[1 1 1] Switch potion generation based on chest type
      (switch `/Game/Enum_imoctezu_PotionChestTypes` (`self.ChestType`)
        (:`NewEnumerator0`
          (bind _returnvalue (`KismetMathLibrary.MakeRotator` 0.0 0.0 _output_get))
          (bind _returnvalue_2 (`KismetMathLibrary.MakeTransform` (0.0 0.0 21.5) _returnvalue (1.0 1.0 1.0)))
          ;;[1 1 1] Create object and save it
          (bind _returnvalue_3 (`AddComponent|NODE_AddStaticMeshComponent-1` :`RelativeTransform` _returnvalue_2 :!label _label))
          (set `self.ItemBeingPlaced` _returnvalue_3))
        (:`NewEnumerator1`
          (bind _returnvalue_4 (`AddComponent|NODE_AddStaticMeshComponent-0` :`RelativeTransform` _returnvalue_2 :!label _label_2))
          (set `self.ItemBeingPlaced` _returnvalue_4))
        (:`NewEnumerator2`
          ;;[1 1 1] Randomize mesh being placed
          (if (> (`KismetMathLibrary.RandomInteger` 100) 50)
            (goto _label)
            (else
              (goto _label_2)))))
      ;;[1 1 1] Decide if it's an object or an object-sized gap
      (if (> (`KismetMathLibrary.RandomFloatInRange` 0.0 100.0) (`self.GapOccurrence`))
        ;;[1 1 1] If it's an object, put it in the right location
        (`SceneComponent.K2_SetRelativeTransform` (`self.ItemBeingPlaced`) (`KismetMathLibrary.MakeTransform` (`KismetMathLibrary.MakeVector` (+ (`KismetMathLibrary.RandomFloatInRange` 0.0 0.0) (`self.CurrentX`)) (`self.CurrentY`) 23.0) _returnvalue (1.0 1.0 1.0)) false false)
        (else
          ;;[1 1 1] If it's a gap, delete the mesh
          (`ActorComponent.K2_DestroyComponent` (`self.ItemBeingPlaced`))))
      ;;[1 1 1] Finally, add Y offset to move to next position
      (set `self.CurrentY` (- (`self.CurrentY`) 13.0)))
    ;;[1 1 1] Add X offset for new row & reset Y position
    (set `self.CurrentX` (+ (`self.CurrentX`) 17.0))
    (set `self.CurrentY` 38.0)))